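; Voxel chunk mesh component that registers itself with nearby static vertex lights in the PS1 horror game.
; On BeginPlay it caches its owning voxel world.
; When a chunk initializes, it converts the chunk bounds to world space and runs a box overlap padded by the scaled voxel size.
; It manually calls HandleBeginOverlap on each BP_StaticVertexLight found, passing itself as the overlapping mesh.
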(event EventBeginPlay
  (bind _asvoxel_world (Utilities|Casting|CastTo (Components|GetOwner)))
  (Variables|Default|SetVoxelWorldRef _asvoxel_world))

(event EventTick
  (params (DeltaSeconds :type Float%20%28single-precision%29)))

(event EventInitChunk
  (params (ChunkLOD :type Byte :default 0) (ChunkBounds :type %20Structure))
  (bind _voxelworldref (Variables|Default|GetVoxelWorldRef))
  (bind _returnvalue (CallFunction|TransformVoxelBoxtoGlobalBox (Variables|Default|GetVoxelWorldRef) ChunkBounds))
  (bind _outactors (Collision|BoxOverlapActors (CallFunction|GetCenter (Utilities|Struct|Make (Class|KismetMathLibrary|FTruncVector (.min _returnvalue)) (Class|KismetMathLibrary|FTruncVector (.max _returnvalue)))) (/ (+ (Math|Conversions|ToVector(Float) (CallFunction|GetSize (Utilities|Struct|Make (Class|KismetMathLibrary|FTruncVector (.min _returnvalue)) (Class|KismetMathLibrary|FTruncVector (.max _returnvalue))))) (* (Variables|Default|GetVoxelSize _voxelworldref) (Transformation|GetActorScale3D _voxelworldref))) 2.0) (Utilities|Array|MakeArray "ObjectTypeQuery2") "/Game/RetroGraphics/Blueprints/BP_StaticVertexLight.BP_StaticVertexLight_C" :!class /Script/Engine.KismetSystemLibrary))
  (for _array_element _outactors
    (bind _asbp_static_vertex_light (Utilities|Casting|CastToBP_StaticVertexLight _array_element))
    (Default|HandleBeginOverlap _asbp_static_vertex_light self)))